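; Resource zone actor that scatters BP_ResourceNode actors within its rotated box area, with zone color and opacity set in construction.
; ReplicateSpawn fills the zone up to a count derived from area, mesh footprint and density, with capped attempts.
; Random points use sphere traces to avoid existing nodes and line traces to align nodes to the ground, with random yaw.
; A looping timer replaces one missing node per cycle, retrying until placed.
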(event Custom|Replicate%20Spawn
  (CallFunction|SpawnNodes)
  (Utilities|FlowControl|DelayUntilNextTick)
  (Utilities|Time|SetTimerbyFunctionName 0 "NodeRespawn" (.noderespawnspawntime (Variables|Default|GetZone%20Info)) true))

(event EventBeginPlay)

(event Collision|EventActorBeginOverlap
  (params (OtherActor :type Actor%20Object%20Reference)))

(event EventTick
  (params (DeltaSeconds :type Float%20%28single-precision%29)))

(fn ConstructionScript
  (bind _zone (Variables|Default|GetZone))
  (bind _zonecolor (Variables|Default|GetZoneColor))
  (bind _returnvalue (Math|Conversions|ToLinearColor(Color) _zonecolor))
  (Rendering|Material|SetScalarParameterValueonMaterials _zone "Opacity" (.a _returnvalue))
  (Rendering|Material|SetVectorParameterValueonMaterials _zone "Color" (Math|Vector|MakeVector (.r _returnvalue) (.g _returnvalue) (.b _returnvalue))))

(fn SpawnNodes
  (bind _boxextent (Collision|GetActorBounds false false))
  (bind _zone_info (Variables|Default|GetZone%20Info))
  (bind _returnvalue (StaticMesh|GetBounds (.nodemesh _zone_info)))
  (bind _output_get (LocalVariables|SetPossibleSpawns (Math|Float|Truncate (* (Math|Float|Floor (Math|Float|SafeDivide (* (.x _boxextent) (.y _boxextent)) (* (.x (.boxextent _returnvalue)) (.y (.boxextent _returnvalue))))) (Math|Float|MapRangeClamped (.resourcedensity (Variables|Default|GetZone%20Info)) 0.0 1e+02 0.0 1.0)))))
  (Variables|Default|SetMaxSpawnAttempts (* _output_get 2))
  (while (and (> (LocalVariables|GetPossibleSpawns) (LocalVariables|GetSpawnCount)) (> (Variables|Default|GetMaxSpawnAttempts) (LocalVariables|GetSpawnAttempts)))
    (LocalVariables|SetSpawnLocation (CallFunction|RandomSpawnLocationfromZone))
    (bind _outhit (Collision|SphereTraceByChannel (+ (LocalVariables|GetSpawnLocation) "0.000000,0.000000,1000.000000") (+ (LocalVariables|GetSpawnLocation) "0.000000,0.000000,-1000.000000") (.sphereradius (StaticMesh|GetBounds (.nodemesh (Variables|Default|GetZone%20Info)))) "TraceTypeQuery1" true 0 "None"))
    (if (not (== (Utilities|GetClass (.hitactor _outhit)) "/Game/ResourceSystem/BP_ResourceNode.BP_ResourceNode_C"))
      (bind _outhit_2 (Collision|LineTraceByChannel (LocalVariables|GetSpawnLocation) (+ (LocalVariables|GetSpawnLocation) "0.000000,0.000000,-1000.000000") "TraceTypeQuery1" true 0 "None"))
      (bind _returnvalue_2 (Game|SpawnActorfromClass "/Game/ResourceSystem/BP_ResourceNode.BP_ResourceNode_C" (Math|Transform|MakeTransform (.location _outhit_2) (Math|Rotator|MakeRotfromZ (.normal _outhit_2)) "1.000000,1.000000,1.000000") "AdjustIfPossibleButAlwaysSpawn" "MultiplyWithRoot" 0 (Variables|Default|GetZone%20Info) 0))
      (Transformation|AddLocalRotation (Variables|/Script/Engine.Actor|GetRootComponent _returnvalue_2) (Math|Rotator|MakeRotator 0.0 0.0 (Math|Random|RandomFloatinRange -1.8e+02 1.8e+02)) false false)
      (Utilities|Array|Add (Variables|Default|GetNodes) _returnvalue_2)
      (Math|Integer|IncrementInt (LocalVariables|GetSpawnCount)
        (:%20%20
          (Math|Integer|IncrementInt (LocalVariables|GetSpawnAttempts))))
      (else
        (Math|Integer|IncrementInt (LocalVariables|GetSpawnAttempts))))))

(fn NodeRespawn
  (for _array_element (Variables|Default|GetNodes)
    (Utilities|IsValid _array_element
      (:Is%20Not%20Valid
        (Utilities|FlowControl|DoOnce false
          (:Completed
            (Utilities|Array|RemoveItem (Variables|Default|GetNodes) _array_element)
            (LocalVariables|SetSpawnLocation (CallFunction|RandomSpawnLocationfromZone) :!label _label)
            (bind _outhit (Collision|SphereTraceByChannel (+ (LocalVariables|GetSpawnLocation) "0.000000,0.000000,1000.000000") (+ (LocalVariables|GetSpawnLocation) "0.000000,0.000000,-1000.000000") (.sphereradius (StaticMesh|GetBounds (.nodemesh (Variables|Default|GetZone%20Info)))) "TraceTypeQuery1" true 0 "ForOneFrame"))
            (if (not (== (Utilities|GetClass (.hitactor _outhit)) "/Game/ResourceSystem/BP_ResourceNode.BP_ResourceNode_C"))
              (bind _outhit_2 (Collision|LineTraceByChannel (LocalVariables|GetSpawnLocation) (+ (LocalVariables|GetSpawnLocation) "0.000000,0.000000,-1000.000000") "TraceTypeQuery1" false 0 "None"))
              (bind _returnvalue (Game|SpawnActorfromClass "/Game/ResourceSystem/BP_ResourceNode.BP_ResourceNode_C" (Math|Transform|MakeTransform (.location _outhit_2) (Math|Rotator|MakeRotfromZ (.normal _outhit_2)) "1.000000,1.000000,1.000000") "AlwaysSpawn" "MultiplyWithRoot" 0 (Variables|Default|GetZone%20Info) 0))
              (Transformation|AddLocalRotation (Variables|/Script/Engine.Actor|GetRootComponent _returnvalue) (Math|Rotator|MakeRotator 0.0 0.0 (Math|Random|RandomFloatinRange -1.8e+02 1.8e+02)) false false)
              (Utilities|Array|Add (Variables|Default|GetNodes) _returnvalue)
              (else
                (goto _label))))))))
  (Utilities|FlowControl|DoOnce false) ; enters at Reset
)

(fn RandomSpawnLocationfromZone
  (bind _zone (Variables|Default|GetZone))
  (bind _zone_2 (Variables|Default|GetZone))
  (bind _returnvalue (Transformation|GetWorldScale _zone))
  (bind _returnvalue_2 (Transformation|GetWorldTransform _zone_2))
  (bind _staticmesh (Variables|/Script/Engine.StaticMeshComponent|GetStaticMesh _zone))
  (bind _returnvalue_3 (StaticMesh|GetBounds _staticmesh))
  (bind _returnvalue_4 (* (.x (.boxextent _returnvalue_3)) (.x _returnvalue)))
  (bind _returnvalue_5 (* (.y (.boxextent _returnvalue_3)) (.y _returnvalue)))
  (return (+ (Math|Vector|RotateVector (Math|Vector|MakeVector (Math|Random|RandomFloatinRange (* _returnvalue_4 -1.0) _returnvalue_4) (Math|Random|RandomFloatinRange (* _returnvalue_5 -1.0) _returnvalue_5) (* (.z (.boxextent _returnvalue_3)) (.z _returnvalue))) (.rotation _returnvalue_2)) (.location _returnvalue_2))))