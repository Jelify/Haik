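; Player Blueprint that handles interaction prompts and triggers interactions with nearby objects.
; Capsule overlaps with BPI_Interaction actors create a prompt widget, and ending such an overlap removes all prompt widgets.
; Interact appends owners of overlapping components tagged "Interactable" to InteractableActors, then sends an interface message to valid entries within range.
; The array is never cleared here, so earlier or duplicate entries can be messaged again.
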(event OnComponentBeginOverlap(CapsuleComponent)
  (params (OverlappedComponent :type Primitive%20Component%20Object%20Reference) (OtherActor :type Actor%20Object%20Reference) (OtherComp :type Primitive%20Component%20Object%20Reference) (OtherBodyIndex :type Integer) (bFromSweep :type Boolean) (SweepResult :type Hit%20Result%20Structure%20%28by%20ref%29))
  (if (Utilities|DoesObjectImplementInterface OtherActor "/Game/Haik/Interaction/BPI_Interaction.BPI_Interaction_C")
    (CallFunction|ShowPrompt)))

(event OnComponentEndOverlap(CapsuleComponent)
  (params (OverlappedComponent :type Primitive%20Component%20Object%20Reference) (OtherActor :type Actor%20Object%20Reference) (OtherComp :type Primitive%20Component%20Object%20Reference) (OtherBodyIndex :type Integer))
  (if (Utilities|DoesObjectImplementInterface OtherActor "/Game/Haik/Interaction/BPI_Interaction.BPI_Interaction_C")
    (CallFunction|HidePrompt)))

(event EventBeginPlay
  (|CallParentFunction) ; This node is disabled and will not be called.\nDrag off pins to build functionality.
)

(event Collision|EventActorBeginOverlap
  (params (OtherActor :type Actor%20Object%20Reference))
  (|CallParentFunction OtherActor))

(event EventTick
  (params (DeltaSeconds :type Float%20%28single-precision%29))
  (|CallParentFunction DeltaSeconds))

(event EventShowPrompt
  (bind _returnvalue (UserInterface|CreateWidget "/Game/Haik/Interaction/WBP_InteractionPrompt.WBP_InteractionPrompt_C"))
  (UserInterface|Viewport|AddtoViewport _returnvalue 0))

(event EventHidePrompt
  (bind _foundwidgets (Widget|GetAllWidgetsOfClass "/Game/Haik/Interaction/WBP_InteractionPrompt.WBP_InteractionPrompt_C" false))
  (for _array_element _foundwidgets
    (Widget|RemovefromParent _array_element)))

(event EventInteract
  (for _array_element (Class|Actor|GetOverlappingComponents)
    (if (Components|ComponentHasTag _array_element "Interactable")
      (Utilities|Array|Add (Variables|Default|GetInteractableActors) (Components|GetOwner _array_element))))
  (for _array_element_2 (Variables|Default|GetInteractableActors)
    (Utilities|IsValid _array_element_2
      (:Is%20Valid
        (if (< (Math|Vector|Distance(Vector) (Transformation|GetActorLocation _array_element_2) (Transformation|GetActorLocation)) 5e+03)
          (Class|BPIInteraction|Interacted(Message) _array_element_2 self))))))

(fn ConstructionScript
  (|CallParentFunction))